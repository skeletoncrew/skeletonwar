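; Game mode for SkeletonWar that maintains a server-side pool of default player names.
; On BeginPlay it loads names from a file, falling back to "Player", and copies them into the available list.
; RepopulatePlayerNames appends another copy of the defaults, suffixed with an incrementing batch number, for future players.
; A nested debug loop prints the whole available list after each addition; name assignment happens outside these graphs.
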(event Custom|RepopulatePlayerNames
  (bind _availableplayernames (Variables|Default|GetAvailablePlayerNames))
  ;[1 1 1] Copy over the default names with an incremented suffix to assign to future players
  (Networking|SwitchHasAuthority
    (:Authority
      (bind _output_get (Variables|Default|SetDefaultPlayerNamesBatch (+ (Variables|Default|GetDefaultPlayerNamesBatch) 1)))
      (for _array_element (Variables|Default|GetDefaultPlayerNames)
        (Utilities|Array|Add _availableplayernames (Utilities|String|Append _array_element (Utilities|String|ToString(Integer) _output_get)))
        (for _array_element_2 _availableplayernames
          (Development|PrintString _array_element_2))))))

(event EventBeginPlay
  (Networking|SwitchHasAuthority
    (:Authority
      ;[1 1 1] Try to read the default names from file, otherwise just set names to "Player"
      (bind _returnvalue (Class|SkeleUtilityFunctionLibrary|GetDefaultPlayerNamesfromFile))
      (if (Utilities|ArrayNotEmpty _returnvalue)
        (Variables|Default|SetDefaultPlayerNames _returnvalue)
        (else
          (Utilities|Array|Add (Variables|Default|GetDefaultPlayerNames) "Player")))
      (Variables|Default|SetAvailablePlayerNames (Variables|Default|GetDefaultPlayerNames)))))

(fn ConstructionScript)