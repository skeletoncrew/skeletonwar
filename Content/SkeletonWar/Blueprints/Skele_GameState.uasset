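; Game state for SkeletonWar that runs the bomb fuses, scoreboard, combat log and match timer, mostly under authority.
; Tick checks the oldest queued bomb and detonates it when its fuse expires, detaching limbs of skeletons in range.
; The bomber gains points per attached limb, or loses them for self-hits, then scoreboard text rebuilds and a hit is logged.
; Time-up only prints "Game over!", and a stopgap timer periodically clears the log.
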(event Custom|DetonateBomb
  (params (BombRef :type Bomb%20BP%20Object%20Reference))
  (bind _owningplayer (Variables|/Game/SkeletonWar/Blueprints/Weapons/BombBP.BombBP_C|GetOwningPlayer BombRef))
  ;[1 1 1] Detonate a bomb
  (Networking|SwitchHasAuthority
    (:Authority
      (if (Utilities|IsValid BombRef)
        (CallFunction|SpawnExplosionParticles (Transformation|GetWorldLocation BombRef))
        (bind _outactors (Actor|GetAllActorsOfClass "/Game/SkeletonWar/Blueprints/PlayerCharacters/Skele_BP.Skele_BP_C"))
        (for _array_element _outactors
          (if (<= (Transformation|GetDistanceTo BombRef _array_element) (Variables|Default|GetBombDamageRange))
            (bind _numlimbsattachedoutput (Default|GetNumLimbsAttached _array_element))
            (for _array_element_2 (Variables|/Game/SkeletonWar/Blueprints/PlayerCharacters/Skele_BP.Skele_BP_C|GetLimbs _array_element)
              (Default|DetachLimbs _array_element_2))
            (bind _asskele_player_state (Utilities|Casting|CastToSkele_PlayerState (Variables|/Script/Engine.Pawn|GetPlayerState _owningplayer)))
            (if (!= _array_element _owningplayer)
              (Default|ModifyPlayerScore _asskele_player_state _numlimbsattachedoutput)
              (else
                (Default|ModifyPlayerScore _asskele_player_state (* _numlimbsattachedoutput -1))))
            (CallFunction|UpdateScoreboard)
            ;[1 1 1] Generate a hit message
            (bind _asskele_player_state_2 (Utilities|Casting|CastToSkele_PlayerState (Variables|/Script/Engine.Pawn|GetPlayerState _array_element)))
            (if (== _asskele_player_state _asskele_player_state_2)
              (Variables|Default|SetBombVictimName "themself")
              (else
                (Variables|Default|SetBombVictimName (Variables|/Game/SkeletonWar/Blueprints/Skele_PlayerState.Skele_PlayerState_C|GetCurrentPlayerName _asskele_player_state_2))))
            (Utilities|Array|Add (Variables|Default|GetCombatLog) (Utilities|String|Append (Utilities|String|Append (Utilities|String|Append (Variables|/Game/SkeletonWar/Blueprints/Skele_PlayerState.Skele_PlayerState_C|GetCurrentPlayerName _asskele_player_state) " blew ") (Variables|Default|GetBombVictimName)) " apart"))))
        (Actor|DestroyActor BombRef)))))

(event Custom|CheckBombs
  (bind _spawnedbombs (Variables|Default|GetSpawnedBombs))
  (bind _item (Utilities|Array|Get(acopy) _spawnedbombs))
  ;[1 1 1] Check for bombs needing to explode
  (Networking|SwitchHasAuthority
    (:Authority
      (if (> (Utilities|Array|Length _spawnedbombs) 0)
        (bind _output_get (Variables|Default|SetTempBombRef _item))
        (if (<= (+ (Variables|/Game/SkeletonWar/Blueprints/Weapons/BombBP.BombBP_C|GetTimeSpawned _item) (Variables|Default|GetBombFuseTime)) (Utilities|Time|GetGameTimeinSeconds))
          (Utilities|Array|RemoveIndex _spawnedbombs)
          (CallFunction|DetonateBomb _output_get))))))

(event Custom|CheckGameTime
  (Networking|SwitchHasAuthority
    (:Authority
      ;[1 1 1] Check game time elapsed
      (if (not (<= (Utilities|Time|GetGameTimeinSeconds) (Variables|Default|GetGameEndTime)))
        (Utilities|FlowControl|Delay 1.0)
        (Development|PrintString "Game over!" true true "(R=0.830000,G=0.012450,B=0.086971,A=1.000000)")))))

(event Custom|SpawnExplosionParticles
  (params (SpawnPos :type Vector :default "0, 0, 0"))
  (bind _returnvalue (Effects|SpawnEmitteratLocation "/Game/StarterContent/Particles/P_Explosion.P_Explosion" SpawnPos))
  (Transformation|SetRelativeScale3D _returnvalue "4.000000,4.000000,4.000000")
  (Class|GameplayStatics|PlaySoundAttached "/Game/StarterContent/Audio/Explosion_Cue.Explosion_Cue" _returnvalue "None" "0, 0, 0" "KeepRelativeOffset" false 1.0))

(event Custom|UpdateScoreboard
  (bind _playerscores (Variables|Default|GetPlayerScores))
  ;[1 1 1] Read all player info to update the scoreboard text
  (Networking|SwitchHasAuthority
    (:Authority
      (bind _outactors (Actor|GetAllActorsOfClass "/Game/SkeletonWar/Blueprints/Skele_PlayerState.Skele_PlayerState_C"))
      (Utilities|Array|Clear _playerscores)
      (for _array_element _outactors
        (Utilities|Array|Add _playerscores (Utilities|String|BuildString(Integer) "" "" (Variables|/Game/SkeletonWar/Blueprints/Skele_PlayerState.Skele_PlayerState_C|GetPlayerScore _array_element) (Utilities|String|Append " : " (Variables|/Game/SkeletonWar/Blueprints/Skele_PlayerState.Skele_PlayerState_C|GetCurrentPlayerName _array_element))))))))

(event EventBeginPlay)

(event EventTick
  (params (DeltaSeconds :type Float%20%28single-precision%29))
  (CallFunction|CheckBombs)
  (CallFunction|CheckGameTime)
  ;[1 1 1] Temporary hackish solution to clear the combat log
  (if (== (Math|Integer|%(Integer) (Math|Float|Floor (Utilities|Time|GetGameTimeinSeconds)) 10) 0)
    (Utilities|FlowControl|Delay 1.1)
    (Utilities|Array|Clear (Variables|Default|GetCombatLog))))

(fn ConstructionScript)