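; Detachable skeleton limb actor that a Skele_BP player picks up on overlap.
; The server attaches it to its preferred socket, falling back to the paired socket or, for legs, to arm sockets, and delays re-pickup after detach.
; OnRep of IsAttached toggles physics and snaps it to or detaches it from the player mesh.
; It also syncs equipped-weapon state with its owner and derives animation state from leg count.
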(event EventActorBeginOverlap
  (params (OtherActor :type Actor%20Object%20Reference))
  (bind _asskele_bp (Utilities|Casting|CastToSkele_BP OtherActor))
  (if (not (Utilities|Array|ContainsItem (Variables|/Game/SkeletonWar/Blueprints/PlayerCharacters/Skele_BP.Skele_BP_C|GetLimbs _asskele_bp) self))
    (CallFunction|PlayerOverlapDetection _asskele_bp)))

(event Custom|Detach%20Limbs
  (bind _limbparentplayer (Variables|Default|GetLimbParentPlayer))
  (bind _actualsocketindex (Variables|Default|GetActualSocketIndex))
  ;[1 1 1] Update variables to tell the server the limb's detached
  (CallFunction|SetLimbVariablesonWeaponDetach)
  (Variables|Default|SetReadyToAttach false)
  (Variables|Default|SetIsAttached false)
  (Utilities|Array|SetArrayElem (Variables|/Game/SkeletonWar/Blueprints/PlayerCharacters/Skele_BP.Skele_BP_C|GetLimbs _limbparentplayer) _actualsocketindex 0)
  (Utilities|Array|SetArrayElem (Variables|/Game/SkeletonWar/Blueprints/PlayerCharacters/Skele_BP.Skele_BP_C|GetHasLimb _limbparentplayer) _actualsocketindex false)
  (Utilities|FlowControl|Delay (Variables|Default|GetLimbPickupDelay))
  (Variables|Default|SetReadyToAttach true))

(event Custom|AttachLimbs
  (params (Player :type Skele%20BP%20Object%20Reference) (SocketIndex :type Integer :default 0))
  (bind _returnvalue (Math|Integer|%(Integer) SocketIndex 2))
  (bind _returnvalue_2 (Math|Integer|%(Integer) SocketIndex 2))
  (bind _returnvalue_3 (* _returnvalue 2))
  (bind _returnvalue_4 (+ _returnvalue_2 1))
  (bind _returnvalue_5 (- _returnvalue_3 1))
  (bind _returnvalue_6 (+ _returnvalue_4 1))
  (bind _returnvalue_7 (+ SocketIndex _returnvalue_5))
  ;[1 1 1] Tries to attach a limb with the given preferred index to the given player
  (bind _asskele_bp (Utilities|Casting|CastToSkele_BP Player))
  (bind _socketinuse (CallFunction|SocketStatus (Variables|/Game/SkeletonWar/Blueprints/PlayerCharacters/Skele_BP.Skele_BP_C|GetHasLimb _asskele_bp) SocketIndex))
  (if _socketinuse
    (if (!= SocketIndex 0)
      (bind _socketinuse_2 (CallFunction|SocketStatus (Variables|/Game/SkeletonWar/Blueprints/PlayerCharacters/Skele_BP.Skele_BP_C|GetHasLimb _asskele_bp) _returnvalue_7))
      (if _socketinuse_2
        ;[1 1 1] Allow legs to go in arm sockets if both leg sockets are full
        (if (>= SocketIndex 3)
          (bind _socketinuse_3 (CallFunction|SocketStatus (Variables|/Game/SkeletonWar/Blueprints/PlayerCharacters/Skele_BP.Skele_BP_C|GetHasLimb _asskele_bp) _returnvalue_4))
          (if _socketinuse_3
            (bind _socketinuse_4 (CallFunction|SocketStatus (Variables|/Game/SkeletonWar/Blueprints/PlayerCharacters/Skele_BP.Skele_BP_C|GetHasLimb _asskele_bp) _returnvalue_6))
            (if (not _socketinuse_4)
              (CallFunction|AttachLimbEvent _returnvalue_6 _asskele_bp))
            (else
              (CallFunction|AttachLimbEvent _returnvalue_4 _asskele_bp))))
        (else
          (CallFunction|AttachLimbEvent _returnvalue_7 _asskele_bp))))
    (else
      (CallFunction|AttachLimbEvent SocketIndex _asskele_bp))))

(event Custom|AttachLimbEvent
  (params (SocketIndex :type Integer :default 0) (ToPlayer :type Skele%20BP%20Object%20Reference))
  ;[1 1 1] Update variables to tell the server the limb's attached
  (Utilities|Array|SetArrayElem (Variables|/Game/SkeletonWar/Blueprints/PlayerCharacters/Skele_BP.Skele_BP_C|GetLimbs ToPlayer) SocketIndex self true)
  (Utilities|Array|SetArrayElem (Variables|/Game/SkeletonWar/Blueprints/PlayerCharacters/Skele_BP.Skele_BP_C|GetHasLimb ToPlayer) SocketIndex true)
  (Variables|Default|SetActualSocketIndex SocketIndex)
  (Variables|Default|SetLimbParentPlayer ToPlayer)
  (Variables|Default|SetIsAttached true))

(event Custom|PlayerOverlapDetection
  (params (OverlappingPlayer :type Skele%20BP%20Object%20Reference))
  (Networking|SwitchHasAuthority
    (:Authority
      (if (Variables|Default|GetReadyToAttach)
        (CallFunction|AttachLimbs OverlappingPlayer (Variables|Default|GetPreferredSocketIndex))))))

(fn ConstructionScript)

(fn GetSocketName
  (bind _preferredsocketindex (Variables|Default|GetPreferredSocketIndex))
  (return (Utilities|Array|Get(acopy) (Variables|Default|GetLimbSocketNames) _preferredsocketindex) _preferredsocketindex))

(fn SocketStatus
  (params (HasLimbArray :type Array%20of%20Booleans) (SocketIndex :type Integer :default 0))
  (return (Utilities|Array|Get(acopy) HasLimbArray SocketIndex)))

(fn OnRepIsAttached
  (bind _isattached (Variables|Default|GetIsAttached))
  (Physics|SetSimulatePhysics (not _isattached))
  (if _isattached
    (Class|Actor|AttachRootComponentto (Variables|/Script/Engine.Character|GetMesh (Variables|Default|GetLimbParentPlayer)) (Utilities|Array|Get(acopy) (Variables|Default|GetLimbSocketNames) (Variables|Default|GetActualSocketIndex)) "SnapToTarget" true)
    (else
      (Class|SceneComponent|DetachfromParent true))))

(fn SetLimbVariablesonWeaponEquip
  (params (Weapon :type Weapon%20Object%20Reference))
  ;[1 1 1] Set variables on limb
  (Variables|Default|SetLimbWeaponEquipped Weapon)
  (Variables|Default|SetLimbHasWeapon true)
  ;[1 1 1] Set Variables on Player
  (bind _asskele_bp (Utilities|Casting|CastToSkele_BP (Variables|Default|GetLimbParentPlayer)))
  (Utilities|FlowControl|Sequence
    (:then_0
      (Variables|/Game/SkeletonWar/Blueprints/PlayerCharacters/Skele_BP.Skele_BP_C|SetPlayerHasWeapon _asskele_bp true))
    (:then_1
      (Variables|/Game/SkeletonWar/Blueprints/PlayerCharacters/Skele_BP.Skele_BP_C|SetWeaponLimb _asskele_bp self))
    (:then_2
      (Variables|/Game/SkeletonWar/Blueprints/PlayerCharacters/Skele_BP.Skele_BP_C|SetEquippedWeapon _asskele_bp (Variables|Default|GetLimbWeaponEquipped)))))

(fn SetLimbVariablesonWeaponDetach
  (if (Variables|Default|GetLimbHasWeapon)
    (Variables|/Game/SkeletonWar/Blueprints/Weapons/Weapon.Weapon_C|SetIsWeaponEquipped (Variables|Default|GetLimbWeaponEquipped) false)
    (Variables|Default|SetLimbHasWeapon false)
    (Variables|/Game/SkeletonWar/Blueprints/PlayerCharacters/Skele_BP.Skele_BP_C|SetPlayerHasWeapon (Variables|Default|GetLimbParentPlayer) false)))

(fn GetAnimationState
  (bind _limbparentplayer (Variables|Default|GetLimbParentPlayer))
  ;[1 1 1] If state has changed
  (if (Variables|/Game/SkeletonWar/Blueprints/PlayerCharacters/Skele_BP.Skele_BP_C|GetPlayerStateChanged _limbparentplayer)
    (Utilities|FlowControl|Sequence
      (:then_0
        (if (Variables|/Game/SkeletonWar/Blueprints/PlayerCharacters/Skele_BP.Skele_BP_C|GetHasNoLegs _limbparentplayer)
          (LocalVariables|SetAnimStateOutput 2)))
      (:then_1
        (if (Variables|/Game/SkeletonWar/Blueprints/PlayerCharacters/Skele_BP.Skele_BP_C|GetHasOneLeg _limbparentplayer)
          (LocalVariables|SetAnimStateOutput 1)))
      (:then_2
        (if (Variables|/Game/SkeletonWar/Blueprints/PlayerCharacters/Skele_BP.Skele_BP_C|GetHasTwoLegs _limbparentplayer)
          (LocalVariables|SetAnimStateOutput 0)))
      (:then_3
        (return (Variables|/Game/SkeletonWar/Blueprints/PlayerCharacters/Skele_BP.Skele_BP_C|GetIsPlayerIdle _limbparentplayer) (LocalVariables|GetAnimStateOutput))))))