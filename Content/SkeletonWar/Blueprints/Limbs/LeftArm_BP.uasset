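; LeftArm_BP is the left arm limb, configured with its own preferred socket and unable to equip weapons.
; On begin play it sets a fixed Speed on its LArm_AnimBP instance.
; Tick polls the parent player's state-changed flag and, while set, plays a looping idle or run animation based on IsIdle.
; The AnimationState switches currently send every listed state to the same animation.
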(event EventBeginPlay
  (|CallParentFunction)
  (bind _aslarm_anim_bp (Utilities|Casting|CastToLArm_AnimBP (Components|SkeletalMesh|GetAnimInstance (Variables|Default|GetSkeletalMesh))))
  (Variables|/Game/SkeletonWar/Animations/LeftArm/LArm_AnimBP.LArm_AnimBP_C|SetSpeed _aslarm_anim_bp 42.0))

(event EventTick
  (params (DeltaSeconds :type Float%20%28single-precision%29))
  (bind (_isidle _animationstate) (CallFunction|GetAnimationState))
  (if (Variables|/Game/SkeletonWar/Blueprints/PlayerCharacters/Skele_BP.Skele_BP_C|GetPlayerStateChanged (Variables|Default|GetLimbParentPlayer))
    (if _isidle
      ;[1 1 1] Change animation
      (switch int _animationstate
        (:0
          _)
        (:1
          _)
        (:2
          _))
      (Components|Animation|PlayAnimation "/Game/SkeletonWar/Animations/LeftArm/LArmIdle_Anim.LArmIdle_Anim" true)
      (else
        (switch int _animationstate
          (:0
            _)
          (:1
            _)
          (:2
            _))
        (Components|Animation|PlayAnimation "/Game/SkeletonWar/Animations/LeftArm/LArmRun_Anim.LArmRun_Anim" true)))))

(fn ConstructionScript
  (|CallParentFunction)
  (Variables|Default|SetPreferredSocketIndex 1)
  (Variables|Default|SetLimbCanEquipWeapon false))