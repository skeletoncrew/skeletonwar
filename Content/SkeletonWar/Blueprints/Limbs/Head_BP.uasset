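; Head limb Blueprint for the skeleton character in SkeletonWar, built on a parent limb class and assigned preferred socket index 0.
; Each tick it checks whether the parent player's state has changed, then loops the head idle or run animation based on the idle flag.
; The animation-state switches send every handled case to the same animation, so the head has no per-state variants.
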(event EventBeginPlay
  (|CallParentFunction))

(event EventActorBeginOverlap
  (params (OtherActor :type Actor%20Object%20Reference)))

(event EventTick
  (params (DeltaSeconds :type Float%20%28single-precision%29))
  (bind (_isidle _animationstate) (CallFunction|GetAnimationState))
  (if (Variables|/Game/SkeletonWar/Blueprints/PlayerCharacters/Skele_BP.Skele_BP_C|GetPlayerStateChanged (Variables|Default|GetLimbParentPlayer))
    (if _isidle
      ;[1 1 1] Change animation
      (switch int _animationstate
        (:0
          _)
        (:1
          _)
        (:2
          _))
      (Components|Animation|PlayAnimation "/Game/SkeletonWar/Animations/Head/HeadIdle_Anim.HeadIdle_Anim" true)
      (else
        (switch int _animationstate
          (:0
            _)
          (:1
            _)
          (:2
            _))
        (Components|Animation|PlayAnimation "/Game/SkeletonWar/Animations/Head/HeadRun_Anim.HeadRun_Anim" true)))))

(fn ConstructionScript
  (|CallParentFunction)
  (Variables|Default|SetPreferredSocketIndex 0))