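; Weapon pickup for skeleton characters that severs other players' limbs.
; When unequipped, overlapping a Skele_BP snaps it to that skeleton's limb 1 hand socket and links weapon and owner.
; A short delay before setting IsEquipped stops it cutting off the arm picking it up.
; While equipped and attacking, overlapping a Limb with a different ParentPlayer calls DetachLimbs on it.
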(event EventBeginPlay)

(event EventActorBeginOverlap
  (params (OtherActor :type Actor%20Object%20Reference))
  (if (Variables|Default|GetIsEquipped)
    (if (Variables|Default|GetIsAttacking)
      (bind _aslimb (Utilities|Casting|CastToLimb OtherActor))
      (if (!= (Variables|/Game/SkeletonWar/Blueprints/Limbs/Limb.Limb_C|GetParentPlayer _aslimb) (Variables|Default|GetParentPlayer))
        (Default|DetachLimbs _aslimb)
        (else
          (Development|PrintString "Limb has same parent"))))
    (else
      (bind _asskele_bp (Utilities|Casting|CastToSkele_BP OtherActor))
      (bind _aslimb_2 (Utilities|Casting|CastToLimb (Utilities|Array|Get(acopy) (Variables|/Game/SkeletonWar/Blueprints/PlayerCharacters/Skele_BP.Skele_BP_C|GetLimbs _asskele_bp) 1)))
      (Variables|/Game/SkeletonWar/Blueprints/PlayerCharacters/Skele_BP.Skele_BP_C|SetWeaponLimb _asskele_bp _aslimb_2)
      (Variables|/Game/SkeletonWar/Blueprints/PlayerCharacters/Skele_BP.Skele_BP_C|SetHasWeapon _asskele_bp true)
      (Variables|/Game/SkeletonWar/Blueprints/PlayerCharacters/Skele_BP.Skele_BP_C|SetEquippedWeapon _asskele_bp self)
      (Class|SceneComponent|Attachto (Variables|/Game/SkeletonWar/Blueprints/Limbs/Limb.Limb_C|GetSkeletalMesh _aslimb_2) "Left_SwordHand" "SnapToTarget" true)
      (Variables|Default|SetParentPlayer _asskele_bp)
      (Utilities|FlowControl|Delay 0.2) ; Delay setting Is Equipped on the weapon to prevent the weapon cutting off the arm trying to pick it up
      (Variables|Default|SetIsEquipped true))))

(event EventTick
  (params (DeltaSeconds :type Float%20%28single-precision%29)))

(fn ConstructionScript
  (Variables|Default|SetIsEquipped false))