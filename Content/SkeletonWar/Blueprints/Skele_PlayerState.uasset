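; Player state for SkeletonWar that holds each player's name and score, with changes made only on the server.
; On BeginPlay it draws a random name from the Skele_GameMode pool and removes it, repopulating the pool when empty.
; ModifyPlayerScore adds a modifier to the score through UpdatePlayerScore.
; Both name assignment at BeginPlay and score changes then ask Skele_GameState to update the scoreboard.
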(event Custom|AssignPlayerInfo
  ;[1 1 1] Assigns the player a name from the array of default names in Skele_GameMode
  (Networking|SwitchHasAuthority
    (:Authority
      (bind _asskele_game_mode (Utilities|Casting|CastToSkele_GameMode (Game|GetGameMode)))
      (if (> (Utilities|Array|Length (Variables|/Game/SkeletonWar/Blueprints/Skele_GameMode.Skele_GameMode_C|GetAvailablePlayerNames _asskele_game_mode)) 0)
        _
        (else
          (Default|RepopulatePlayerNames _asskele_game_mode)))
      (bind _output_get (Variables|Default|SetPlayerNameIndex (Math|Random|RandomInteger (Utilities|Array|Length (Variables|/Game/SkeletonWar/Blueprints/Skele_GameMode.Skele_GameMode_C|GetAvailablePlayerNames _asskele_game_mode)))))
      (Variables|Default|SetCurrentPlayerName (Utilities|Array|Get(acopy) (Variables|/Game/SkeletonWar/Blueprints/Skele_GameMode.Skele_GameMode_C|GetAvailablePlayerNames _asskele_game_mode) _output_get))
      (Utilities|Array|RemoveIndex (Variables|/Game/SkeletonWar/Blueprints/Skele_GameMode.Skele_GameMode_C|GetAvailablePlayerNames _asskele_game_mode) _output_get))))

(event Custom|UpdatePlayerScore
  (params (NewScore :type Integer :default 0))
  (Networking|SwitchHasAuthority
    (:Authority
      (Variables|Default|SetPlayerScore NewScore))))

(event EventBeginPlay
  (Networking|SwitchHasAuthority
    (:Authority
      (CallFunction|AssignPlayerInfo)
      (bind _asskele_game_state (Utilities|Casting|CastToSkele_GameState (Game|GetGameState)))
      (Default|UpdateScoreboard _asskele_game_state))))

(event EventTick
  (params (DeltaSeconds :type Float%20%28single-precision%29)))

(fn ConstructionScript)

(fn ModifyPlayerScore
  (params (Modifier :type Integer :default 0))
  (CallFunction|UpdatePlayerScore (+ (Variables|Default|GetPlayerScore) Modifier))
  (bind _asskele_game_state (Utilities|Casting|CastToSkele_GameState (Game|GetGameState)))
  (Default|UpdateScoreboard _asskele_game_state))